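; Manager actor for an AI rat simulation that populates the level with rats and food and shows a statistics widget.
; A looping timer and the F key spawn food; number keys spawn adult Alpha, Beta or Female rats, with player input enabled on BeginPlay.
; Spawns use random reachable navmesh points around a fixed origin.
; New rats start Roaming, with gameplay tags for role and state and a material per role.
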(event `self.ReceiveBeginPlay`
  (`self.EnableInput` (`GameplayStatics.GetPlayerController` 0))
  (`KismetSystemLibrary.K2_SetTimer` null "SpawnFood" (`self.FoodSpawnTimeRate`) true)
  (bind _returnvalue (`|CreateWidget` "/Game/StatisticsWidget.StatisticsWidget_C"))
  (`UserWidget.AddToViewport` _returnvalue 0))

(event `Key|One`
  (params (Key :type "Key Structure"))
  (:`Pressed`
    (`self.SpawnRat` (struct :`TagName` "Role.Alpha"))))

(event `Key|Two`
  (params (Key :type "Key Structure"))
  (:`Pressed`
    (`self.SpawnRat` (struct :`TagName` "Role.Beta"))))

(event `Key|F`
  (params (Key :type "Key Structure"))
  (:`Pressed`
    (`self.SpawnFood`)))

(event `Key|Three`
  (params (Key :type "Key Structure"))
  (:`Pressed`
    (`self.SpawnRat` (struct :`TagName` "Role.Female"))))

(fn `SpawnFood`
  (bind (_returnvalue_location _returnvalue_rotation) (`KismetMathLibrary.BreakTransform` (`SceneComponent.K2_GetComponentToWorld` (`self.DefaultSceneRoot`))))
  (`|SpawnActorFromClass` "/Game/BP_Food.BP_Food_C" (`KismetMathLibrary.MakeTransform` (`NavigationSystemV1.K2_GetRandomReachablePointInRadius` (`KismetMathLibrary.MakeVector` 1500.0 2000.0 100.0) 2000.0 null null) _returnvalue_rotation (0.5 0.5 1.0)) "AdjustIfPossibleButAlwaysSpawn" "OverrideRootScale" null null))

(fn `SpawnRat`
  (params (Role :type "GameplayTag Structure") (Child :type Boolean))
  (bind (_returnvalue_location _returnvalue_rotation) (`KismetMathLibrary.BreakTransform` (`SceneComponent.K2_GetComponentToWorld` (`self.DefaultSceneRoot`))))
  (bind _returnvalue (`|SpawnActorFromClass` "/Game/BP_Rat.BP_Rat_C" (`KismetMathLibrary.MakeTransform` (`NavigationSystemV1.K2_GetRandomReachablePointInRadius` (`KismetMathLibrary.MakeVector` 1500.0 2000.0 90.0) 1000.0 null null) _returnvalue_rotation) "AdjustIfPossibleButAlwaysSpawn" "OverrideRootScale" null (struct) (struct) null))
  (set `/Game/BP_Rat.Child` Child _returnvalue)
  (bind _output_get (set `/Game/BP_Rat.ActorRole` Role _returnvalue))
  (set `/Game/BP_Rat.ActorState` (struct :`TagName` "State.Roaming") _returnvalue)
  (`|SwitchGameplayTag` _output_get
    (:`Role.Alpha`
      (bind _mesh (`Character.Mesh` _returnvalue))
      (`PrimitiveComponent.SetMaterial` _mesh 0 "/Game/Materials/M_Metal_Burnished_Steel.M_Metal_Burnished_Steel"))
    (:`Role.Beta`
      (`PrimitiveComponent.SetMaterial` _mesh 0 "/Game/Materials/M_Ground_Gravel.M_Ground_Gravel"))
    (:`Role.Female`
      (`PrimitiveComponent.SetMaterial` _mesh 0 "/Game/Materials/M_Metal_Copper.M_Metal_Copper"))))

(fn `UserConstructionScript`)