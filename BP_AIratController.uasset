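; AI controller for BP_Rat that drives BT_AIrat through a gameplay-tag actor state.
; While roaming, perception of non-child rats sets state by role: Alphas chase, Betas evade Alphas, Females evade Alphas by chance.
; Looping timers switch between food search and roaming on Food and Health, and copy state changes to the blackboard, rerunning the tree.
; Roam and FoodSearch events hold separate movement logic, partly disconnected.
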(event `self.ReceiveBeginPlay`
  (bind _listenerstimerate (`self.ListenersTimeRate`))
  (`KismetSystemLibrary.DelayUntilNextTick`)
  (bind _asbp_airat_game (cast `/Game/BP_AIratGame` (`GameplayStatics.GetGameMode`)))
  (set `self.CustomGameMode` _asbp_airat_game)
  (bind _asbp_rat (cast `/Game/BP_Rat` (`self.K2_GetPawn`)))
  (set `self.SpawnedRatAI` _asbp_rat)
  (`KismetSystemLibrary.K2_SetTimer` null "StateTag Listener" _listenerstimerate true)
  (`KismetSystemLibrary.K2_SetTimer` null "HealthFoodListener" _listenerstimerate true)
  (`self.RunBehaviorTree` "/Game/BT_AIrat.BT_AIrat"))

(event `self.AIPerception.OnTargetPerceptionUpdated`
  (params (Actor :type "Actor Object Reference") (Stimulus :type "AIStimulus Structure"))
  (bind (_age _expirationage _strength _stimuluslocation _receiverlocation _tag _bsuccessfullysensed) (break `AIStimulus` Stimulus))
  (bind _asbp_rat (cast `/Game/BP_Rat` Actor))
  (if (and (== (`/Game/BP_Rat.ActorState` (`self.SpawnedRatAI`)) (struct :`TagName` "State.Roaming")) (!= (`/Game/BP_Rat.Child` _asbp_rat) true))
    (`|SwitchGameplayTag` (`/Game/BP_Rat.ActorRole` (`self.SpawnedRatAI`))
      (:`Role.Beta`
        (bind _returnvalue (== (`/Game/BP_Rat.ActorRole` _asbp_rat) (struct :`TagName` "Role.Alpha")))
        (if (and _bsuccessfullysensed _returnvalue)
          (set `/Game/BP_Rat.ActorState` (struct :`TagName` "State.Evading") (`self.SpawnedRatAI`))))
      (:`Role.Alpha`
        (if _bsuccessfullysensed
          (set `/Game/BP_Rat.ActorState` (struct :`TagName` "State.Chasing") (`self.SpawnedRatAI`))))
      (:`Role.Female`
        (if (and _returnvalue _bsuccessfullysensed)
          (if (<= (`KismetMathLibrary.RandomFloat`) (`self.PercentageFemaleEvade`))
            (set `/Game/BP_Rat.ActorState` (struct :`TagName` "State.Evading") (`self.SpawnedRatAI`))))))))

(event `Roam`
  (bind _returnvalue (`self.K2_GetActorLocation`))
  (bind _randomlocation (`NavigationSystemV1.K2_GetRandomReachablePointInRadius` _returnvalue 1000.0 null null))
  ;[1 1 1] AI roam
  (`self.SetControlRotation` (`KismetMathLibrary.FindLookAtRotation` _returnvalue _randomlocation))
  (`|AIMoveTo` (`self.K2_GetPawn`) _randomlocation null
    (:`OnSuccess`
      _)
    (:`OnFail`
      _))
  (`self.Roam`))

(event `FoodSearch`
  (for _array_element (`AIPerceptionComponent.GetPerceivedActors` (`self.AIPerception`) "/Script/AIModule.AISense_Sight")
    (if (== (`GameplayStatics.GetObjectClass` _array_element) "/Game/BP_Food.BP_Food_C")
      (break))))

(fn `HealthFoodListener`
  (bind _spawnedratai (`self.SpawnedRatAI`))
  (bind _food (`/Game/BP_Rat.Food` _spawnedratai))
  (bind _returnvalue (<= _food 1.0))
  (bind _returnvalue_2 (<= (`/Game/BP_Rat.Health` _spawnedratai) 1.0))
  (if (== _food 0.0)
    (set `/Game/BP_Rat.ActorState` (struct :`TagName` "State.SearchingForFood") (`self.SpawnedRatAI`) :!label _label)
    (elif (`BlueprintGameplayTagLibrary.MatchesTag` (`/Game/BP_Rat.ActorState` (`self.SpawnedRatAI`)) (struct :`TagName` "State.Roaming"))
      (if _returnvalue
        (goto _label)
        (elif _returnvalue_2
          (goto _label)))
      (elif (`BlueprintGameplayTagLibrary.MatchesTag` (`/Game/BP_Rat.ActorState` (`self.SpawnedRatAI`)) (struct :`TagName` "State.SearchingForFood"))
        (if (and (!= _returnvalue_2 true) (!= _returnvalue true))
          (set `/Game/BP_Rat.ActorState` (struct :`TagName` "State.Roaming") (`self.SpawnedRatAI`)))))))

(fn `StateTag Listener`
  (bind _spawnedratai (`self.SpawnedRatAI`))
  (bind _actorstate (`/Game/BP_Rat.ActorState` _spawnedratai))
  (if (!= _actorstate (`self.ActorStateArchive`))
    (bind _output_get (set `self.ActorStateArchive` _actorstate))
    (if (== _output_get (struct :`TagName` "State.SearchingForFood"))
      (`/Game/BP_Rat.PerceptionOnOff` _spawnedratai true))
    (bind _blackboardcomponent (`self.UseBlackboard` "/Game/BB_AIrat.BB_AIrat"))
    (`BlackboardComponent.SetValueAsName` _blackboardcomponent "ActorState" (`BlueprintGameplayTagLibrary.GetTagName` (`/Game/BP_Rat.ActorState` (`self.SpawnedRatAI`))))
    (`self.RunBehaviorTree` "/Game/BT_AIrat.BT_AIrat")))

(fn `UserConstructionScript`)