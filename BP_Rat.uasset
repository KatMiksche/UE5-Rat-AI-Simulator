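; Rat pawn for a population simulation, player or AI driven, with food, health, limited lifespan and a status widget.
; Looping timers drain food and heal health, with starvation causing damage.
; Overlaps let non-foraging adult Alphas fight Alphas or Betas or impregnate Females, then AI rats flee and fighters or maters briefly lose sight.
; Pregnant Females change material, drop their perception stimulus, and later spawn random-role children through the game mode.
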(event `InputAxis|MoveForward`
  (params (AxisValue :type "Float (single-precision)"))
  (`self.AddMovementInput` (`self.GetActorForwardVector`) AxisValue))

(event `InputAxis|MoveRight`
  (params (AxisValue :type "Float (single-precision)"))
  (`self.AddMovementInput` (`self.GetActorRightVector`) AxisValue))

(event `self.ReceiveTick`
  (params (DeltaSeconds :type "Float (single-precision)"))
  (bind _returnvalue (`self.ConsumeMovementInputVector`))
  (`self.K2_AddActorLocalOffset` (* _returnvalue DeltaSeconds) true)
  (`self.UpdateHealthFoodWidget`))

(event `self.ReceiveBeginPlay`
  (bind _playerhealthoverride (`self.PlayerHealthOverride`))
  (`|ExecutionSequence`
    (:`then_0`
      (bind _asbp_airat_game (cast `/Game/BP_AIratGame` (`GameplayStatics.GetGameMode`)))
      (set `self.CustomGameMode` _asbp_airat_game)
      (bind _asbp_airat_controller (cast `/Game/BP_AIratController` (`self.GetController`)))
      (set `self.CustomController` _asbp_airat_controller))
    (:`then_1`
      (if (not (`self.IsPlayerControlled`))
        (`KismetSystemLibrary.DelayUntilNextTick`)
        (set `CharacterMovementComponent.MaxWalkSpeed` (`/Game/BP_AIratGame.RatsSpeed` (`self.CustomGameMode`)) (`self.CharacterMovement`))))
    (:`then_2`
      (add `self.SuccessfulPregnancy` (delegate `SuccessfulPregnancy_Event_0`)))
    (:`then_3`
      (if (and (`self.IsPlayerControlled`) (!= _playerhealthoverride 0.0))
        (bind _output_get (set `self.MaxHealth` _playerhealthoverride))
        (set `self.Health` _output_get)))
    (:`then_4`
      (`KismetSystemLibrary.K2_SetTimer` null "DecreaseFood" (`self.FoodDepletionTimeRate`) true)
      (`KismetSystemLibrary.K2_SetTimer` null "IncreaseHealth" (`self.HealingTimeRate`) true)
      (`KismetSystemLibrary.Delay` (`self.ChildProtectedTime`))
      (set `self.Child` false)
      (`KismetSystemLibrary.Delay` (* (`self.LifeSpanInMinutes`) 60.0))
      (`self.K2_DestroyActor`))))

(event `SuccessfulPregnancy_Event_0`
  (`KismetSystemLibrary.Delay` (`self.LengthOfPregnancy`))
  (`self.GivingBirth`))

(event `self.ReceiveActorBeginOverlap`
  (params (OtherActor :type "Actor Object Reference"))
  (if (== (`GameplayStatics.GetObjectClass` OtherActor) "BP_Rat_C")
    (bind _asbp_rat (cast `/BP_Rat` OtherActor))
    (if (and (!= (`/BP_Rat.Child` _asbp_rat) true) (== (`self.ActorRole`) (struct :`TagName` "Role.Alpha")) (!= (`self.ActorState`) (struct :`TagName` "State.SearchingForFood")) (!= (`self.Child`) true))
      (`|SwitchGameplayTag` (`/BP_Rat.ActorRole` _asbp_rat)
        (:`Role.Alpha`
          (`self.FightWithAlpha` _asbp_rat)
          (`self.RunOppositeDirection` _asbp_rat :!label _label)
          (`self.RunOppositeDirection` _asbp_rat self))
        (:`Role.Beta`
          (`self.FightWithBeta` _asbp_rat)
          (goto _label))
        (:`Role.Female`
          (if (not (`/BP_Rat.Pregnancy` _asbp_rat))
            (`self.MateWithFemale` _asbp_rat)
            (goto _label)))))))

(event `PerceptionOnOff`
  (params (OnOff :type Boolean))
  (if (not (`self.IsPlayerControlled`))
    (`AIPerceptionComponent.SetSenseEnabled` (`/Game/BP_AIratController.AIPerception` (`self.CustomController`)) "/Script/AIModule.AISense_Sight" OnOff)
    (if (not OnOff)
      (`KismetSystemLibrary.Delay` (`self.LengthOfBlindnessAfterFight`))
      (`self.PerceptionOnOff` true))))

(fn `DecreaseFood`
  (bind _food (`self.Food`))
  (if (== 0.0 _food)
    (`self.DecreaseHealth` 1.0)
    (else
      (set `self.Food` (`KismetMathLibrary.FClamp` (- _food 1.0) 0.0 (`self.MaxFood`))))))

(fn `DecreaseHealth`
  (params (Hit :type "Float (double-precision)"))
  (bind _returnvalue (`KismetMathLibrary.FClamp` (- (`self.Health`) Hit) 0.0 (`self.MaxHealth`)))
  (if (<= _returnvalue 0.0)
    (`self.K2_DestroyActor`)
    (else
      (set `self.Health` _returnvalue))))

(fn `FightWithAlpha`
  (params (ActorOtherAlpha :type "/BP_Rat Object Reference"))
  (for _array_element (`|MakeArray` self ActorOtherAlpha :!type "/BP_Rat Object Reference")
    (`self.DecreaseHealth` _array_element 1.0)
    (`self.PerceptionOnOff` _array_element false)))

(fn `FightWithBeta`
  (params (ActorBeta :type "/BP_Rat Object Reference"))
  (`|ExecutionSequence`
    (:`then_0`
      (`self.DecreaseHealth` ActorBeta 2.0)
      (`self.PerceptionOnOff` ActorBeta false))
    (:`then_1`
      (`self.DecreaseFood`)
      (`self.PerceptionOnOff` false))))

(fn `GivingBirth`
  (locals (MinOffsprings :type Integer :default 5))
  (bind _returnvalue (`KismetMathLibrary.RandomFloatInRange` 0.0 1.0))
  (bind _customgamemode (`self.CustomGameMode`))
  (`|ExecutionSequence`
    (:`then_0`
      ;[1 1 1] Reset Female
      (`|AddComponentByClass` "/Script/AIModule.AIPerceptionStimuliSourceComponent"))
    (:`then_1`
      (`PrimitiveComponent.SetMaterial` (`self.Mesh`) 0 "/Game/Materials/M_Water_Lake.M_Water_Lake"))
    (:`then_2`
      (set `self.FoodDepletionTimeRate` (* (`self.FoodDepletionTimeRate`) 0.5)))
    (:`then_3`
      (set `self.Pregnancy` false))
    (:`then_4`
      ;[1 1 1] Spawning new rats
      (for _ (range 1 (+ (`KismetMathLibrary.RandomIntegerInRange` (`local.MinOffsprings`) (`self.MaxOffsprings`)) 1))
        (if (< _returnvalue (`self.ChanceOfFemale`))
          (`/Game/BP_AIratGame.SpawnRat` _customgamemode (struct :`TagName` "Role.Alpha") true)
          (elif (> _returnvalue (- 1.0 (`self.ChanceOfMale`)))
            (`/Game/BP_AIratGame.SpawnRat` _customgamemode (struct :`TagName` "Role.Female") true)
            (else
              (`/Game/BP_AIratGame.SpawnRat` _customgamemode (struct :`TagName` "Role.Beta") true))))))))

(fn `IncreaseHealth`
  (if (!= (`self.Food`) 0.0)
    (set `self.Health` (`KismetMathLibrary.FClamp` (+ (`self.Health`) 1.0) 0.0 (`self.MaxHealth`)))))

(fn `MateWithFemale`
  (params (ActorFemale :type "/BP_Rat Object Reference"))
  (`|ExecutionSequence`
    (:`then_0`
      ;[1 1 1] Female
      (`ActorComponent.K2_DestroyComponent` (`/BP_Rat.AIPerceptionStimuliSource` ActorFemale)))
    (:`then_1`
      (`PrimitiveComponent.SetMaterial` (`Character.Mesh` ActorFemale) 0 "/Game/Materials/MI_Solid_Blue.MI_Solid_Blue"))
    (:`then_2`
      (set `/BP_Rat.FoodDepletionTimeRate` (* (`/BP_Rat.FoodDepletionTimeRate` ActorFemale) 2.0) ActorFemale))
    (:`then_3`
      (set `/BP_Rat.Pregnancy` true ActorFemale))
    (:`then_4`
      (`self.SuccessfulPregnancy` ActorFemale))
    (:`then_5`
      ;[1 1 1] Alpha
      (`self.DecreaseFood`))
    (:`then_6`
      (`self.PerceptionOnOff` false))))

(fn `RunOppositeDirection`
  (params (OtherActor :type "/BP_Rat Object Reference"))
  (bind _returnvalue (`self.K2_GetActorLocation`))
  (if (not (`self.IsPlayerControlled`))
    (`AIBlueprintHelperLibrary.SimpleMoveToLocation` (`self.GetController`) (+ _returnvalue (* (`KismetMathLibrary.GetForwardVector` (`KismetMathLibrary.FindLookAtRotation` _returnvalue (`self.K2_GetActorLocation` OtherActor))) -500.0)))
    (set `self.ActorState` (struct :`TagName` "State.Roaming"))))

(fn `UpdateHealthFoodWidget`
  (bind _returnvalue (`KismetStringLibrary.Concat_StrStr` (`KismetStringLibrary.Conv_NameToString` (`BlueprintGameplayTagLibrary.GetTagName` (`self.ActorRole`))) ", " (`KismetStringLibrary.Conv_NameToString` (`BlueprintGameplayTagLibrary.GetTagName` (`self.ActorState`)))))
  (bind _ashealth_food_widget (cast `/Game/HealthFoodWidget` (`WidgetComponent.GetUserWidgetObject` (`self.Bars`))))
  (if (`self.Child`)
    (set `/Game/HealthFoodWidget.TextWidget` (`KismetStringLibrary.Concat_StrStr` "CHILD: " _returnvalue) _ashealth_food_widget)
    (else
      (set `/Game/HealthFoodWidget.TextWidget` _returnvalue _ashealth_food_widget)))
  (set `/Game/HealthFoodWidget.FoodInWidget` (/ (`self.Food`) (`self.MaxFood`)) _ashealth_food_widget)
  (set `/Game/HealthFoodWidget.HealthInWidget` (/ (`self.Health`) (`self.MaxHealth`)) _ashealth_food_widget))

(fn `UserConstructionScript`)